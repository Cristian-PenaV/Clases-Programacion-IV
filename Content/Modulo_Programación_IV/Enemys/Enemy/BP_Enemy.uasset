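; Enemy pawn Blueprint that patrols waypoints and chases the player when it sees a pawn.
; Patrol starts at BeginPlay and loops through the Waypoints array, advancing on each successful AIMoveTo.
; PawnSensing starts a chase toward player 0 without checking which pawn was seen, and a one-second retriggerable delay resumes patrol after sightings stop.
; A random-point wander event is defined but never called in this graph.
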(event OnSeePawn(PawnSensing)
  (params (Pawn :type Pawn%20Object%20Reference))
  ;[0 1 0.7349] Si veo al Jugador
  (Utilities|FlowControl|Sequence
    (:then_0
      (Development|PrintString "Voy por el player")
      (CallFunction|ChasePlayer))
    (:then_1
      (Utilities|FlowControl|RetriggerableDelay 1.0)
      (CallFunction|FollowWaypoints))))

(event Custom|Chase%20Player
  ;[1 0 0.5251] Seguir al jugador
  (AI|AIMoveTo self "0, 0, 0" (Game|GetPlayerCharacter 0) 5.0 false))

(event Custom|Follow%20Waypoints
  (bind _waypoints (Variables|Default|GetWaypoints))
  ;[0.4106 0 1] Patrullar
  (AI|AIMoveTo self "0, 0, 0" (Utilities|Array|Get(acopy) _waypoints (Variables|Default|GetCurrent%20Waypoint)) 5.0 false
    (:OnSuccess
      (bind _result (Math|Integer|IncrementInt (Variables|Default|GetCurrent%20Waypoint))
        (:%20%20
          (if (>= _result (Utilities|Array|Length _waypoints))
            (Variables|Default|SetCurrent%20Waypoint 0))
          (CallFunction|FollowWaypoints))))))

(event Custom|Follow%20Random%20Point
  ;[1 0.1028 0] Patrullar punto Aleatorio
  (AI|AIMoveTo self (.RandomLocation (AI|Navigation|GetRandomReachablePointinRadius (Transformation|GetActorLocation) 1e+02 0 0)) 0 5.0 false
    (:then
      (CallFunction|FollowRandomPoint))))

(event EventBeginPlay
  (CallFunction|FollowWaypoints))

(fn ConstructionScript)